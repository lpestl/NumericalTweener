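; BP_TweenDemoBall is a demo ball that endlessly pulses its red emissive glow and bobs up and down using a selectable easing type.
; On BeginPlay it finds the level's BP_Tweener and creates a dynamic material instance for its sphere.
; Paired tweens drive the glow and height variables back and forth, looping through finish callbacks.
; Tick applies both values to the material and the sphere's relative location.
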(event `self.ReceiveBeginPlay`
  (`|ExecutionSequence`
    (:`then_0`
      ;[1 1 1] Found and save TweenManager instance (Tweener)
      (bind _returnvalue (`GameplayStatics.GetActorOfClass` "/Game/NumericalTweener/Blueprints/Tweener/BP_Tweener.BP_Tweener_C"))
      (`/Engine/EditorBlueprintResources/StandardMacros.IsValid` _returnvalue
        (:`Is Valid`
          (set `self.TweenManager` _returnvalue))))
    (:`then_1`
      ;[1 1 1] Create and save Dynamic Material instance
      (bind _returnvalue_2 (`PrimitiveComponent.CreateDynamicMaterialInstance` (`self.Sphere`) 0 "/Game/DemoRoom/Materials/MI_EmissiveTween.MI_EmissiveTween" "None"))
      (bind _output_get (set `self.EmissiveMaterial` _returnvalue_2))
      (`MaterialInstanceDynamic.SetVectorParameterValue` _output_get "Color" (struct :`R` 1.0 :`A` 1.0))
      (`MaterialInstanceDynamic.SetScalarParameterValue` _output_get "Volume" (`self.emissiveVolume`)))
    (:`then_2`
      ;[1 1 1] Create 1.5 sec Tween for emissive
      (`Tweener.AddEaseTween` (`self.TweenManager`) (`self.emissiveVolume`) 1.0 1.5 (`self.TweenType`) (delegate `OnFinish`) :!label _label)
      (`Tweener.AddEaseTween` :`self` (`self.TweenManager`) :`Var` (`self.positionZ`) :`To` 250.0 :`Time` 1.5 :`Transition` (`self.TweenType`)))))

(event `OnFinishAgain`
  (goto _label))

(event `OnFinish`
  ;[1 1 1] Callback and Tween again back
  (`Tweener.AddEaseTween` (`self.TweenManager`) (`self.emissiveVolume`) 0.0 1.5 (`self.TweenType`) (delegate `OnFinishAgain`))
  (`Tweener.AddEaseTween` :`self` (`self.TweenManager`) :`Var` (`self.positionZ`) :`To` 0.0 :`Time` 1.5 :`Transition` (`self.TweenType`)))

(event `self.ReceiveTick`
  (params (DeltaSeconds :type "Float (single-precision)"))
  (`MaterialInstanceDynamic.SetScalarParameterValue` (`self.EmissiveMaterial`) "Volume" (`self.emissiveVolume`))
  (`SceneComponent.K2_SetRelativeLocation` (`self.Sphere`) (`KismetMathLibrary.MakeVector` 0.0 0.0 (`self.positionZ`)) false false))

(fn `UserConstructionScript`)