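; Easing function library for the Numerical Tweener, mapping time, start value, change and duration (T, B, C, D) to an interpolated value.
; Linear, sine in, out and in-out, and cubic ease-in each evaluate a Penner-style formula through a Math Expression node.
; EaseOutCubic is a stub returning zero, and EaseInOutCubic is empty with no inputs or output.
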(fn Linear
  (params (t :type Float%20%28single-precision%29) (b :type Float%20%28single-precision%29) (c :type Float%20%28single-precision%29) (d :type Float%20%28single-precision%29))
  (return (|(((c*t)/d)+b) c t d b)))

(fn EaseinSine
  (params (t :type Float%20%28single-precision%29) (b :type Float%20%28single-precision%29) (c :type Float%20%28single-precision%29) (d :type Float%20%28single-precision%29))
  (return (|((c+b)-(c*(cos((((t/d)*p)/2))))) t d (Math|Trig|GetPI) c b)))

(fn EaseOutSine
  (params (t :type Float%20%28single-precision%29) (b :type Float%20%28single-precision%29) (c :type Float%20%28single-precision%29) (d :type Float%20%28single-precision%29))
  (return (|((c*(sin(((t/d)*(p/2)))))+b) c t d (Math|Trig|GetPI) b)))

(fn EaseinOutSine
  (params (t :type Float%20%28single-precision%29) (b :type Float%20%28single-precision%29) (c :type Float%20%28single-precision%29) (d :type Float%20%28single-precision%29))
  (return (|(b-((c/2)*((cos(((p*t)/d)))-1))) b c (Math|Trig|GetPI) t d)))

(fn EaseinCubic
  (params (t :type Float%20%28single-precision%29) (b :type Float%20%28single-precision%29) (c :type Float%20%28single-precision%29) (d :type Float%20%28single-precision%29))
  (return (|((((c*t)*t)*t)+b) c (/ t d) b)))

(fn EaseOutCubic
  (params (t :type Float%20%28single-precision%29) (b :type Float%20%28single-precision%29) (c :type Float%20%28single-precision%29) (d :type Float%20%28single-precision%29))
  (return 0.0))

(fn EaseinOutCubic)